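; Enemy spawner actor whose Blueprint graph only displays the remaining spawn cooldown as text in the world.
; Each Tick reads SpawnCooldownManager and, while the cooldown is not nearly zero, writes it to TextRender, blanking the text once under one second remains.
; No spawning logic appears in this graph; BeginPlay, overlap and the construction script are empty.
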(event EventBeginPlay)

(event Collision|EventActorBeginOverlap
  (params (OtherActor :type Actor%20Object%20Reference)))

(event EventTick
  (params (DeltaSeconds :type Float%20%28single-precision%29))
  (bind _spawncooldownmanager (Variables|Default|GetSpawnCooldownManager))
  (bind _returnvalue (Class|CCooldownManager|GetRemainingCooldown _spawncooldownmanager))
  (if (not (Math|Float|NearlyEqual(Float) _returnvalue 0.0 1e-06))
    (if (< _returnvalue 1.0)
      (Rendering|Components|TextRender|SetText (Variables|Default|GetTextRender) (Utilities|Text|MakeLiteralText ""))
      (else
        (Rendering|Components|TextRender|SetText (Variables|Default|GetTextRender) (Utilities|Text|ToText(Float) _returnvalue "HalfToEven" false true 1 324 0 0))))))

(fn ConstructionScript)