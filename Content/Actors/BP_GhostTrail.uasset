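; BP_GhostTrail is a short-lived afterimage actor that shows a frozen, tinted copy of a skeletal mesh.
; On BeginPlay, Init gives its PoseableMesh the source component's mesh and applies an offset transform.
; Each material slot gets MI_GhostTrail and a dynamic instance colored by InColor, then the source's current pose is copied once.
; The actor destroys itself after RemoveTime.
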(event EventBeginPlay
  (CallFunction|Init (Variables|Default|GetInComponentToCopy))
  (Utilities|FlowControl|Delay (Variables|Default|GetRemoveTime))
  (Actor|DestroyActor))

(event Collision|EventActorBeginOverlap
  (params (OtherActor :type Actor%20Object%20Reference)))

(event EventTick
  (params (DeltaSeconds :type Float%20%28single-precision%29)))

(fn ConstructionScript)

(fn Init
  (params (InSkeletalMeshComp :type Skeletal%20Mesh%20Component%20Object%20Reference))
  (Utilities|IsValid InSkeletalMeshComp
    (:Is%20Valid
      (Class|SkinnedMeshComponent|SetSkeletalMesh (Variables|Default|GetPoseableMesh) (Variables|/Script/Engine.SkinnedMeshComponent|GetSkeletalMesh InSkeletalMeshComp) true)
      (Transformation|SetRelativeTransform (Variables|Default|GetPoseableMesh) (Variables|Default|GetSkeletalMeshOffset) false true)
      (for (_array_element _array_index) (Rendering|Material|GetMaterials (Variables|Default|GetPoseableMesh))
        (Rendering|Material|SetMaterial (Variables|Default|GetPoseableMesh) _array_index "/Game/Materials/MI_GhostTrail.MI_GhostTrail")
        (bind _returnvalue (Rendering|Material|CreateDynamicMaterialInstance _array_element "None" :!class /Script/Engine.KismetMaterialLibrary))
        (Rendering|Material|SetVectorParameterValue _returnvalue "Color" (Variables|Default|GetInColor) :!class /Script/Engine.MaterialInstanceDynamic)
        (Rendering|Material|SetMaterial (Variables|Default|GetPoseableMesh) _array_index _returnvalue))
      (Class|PoseableMeshComponent|CopyPosefromSkeletalComponent (Variables|Default|GetPoseableMesh) InSkeletalMeshComp))))