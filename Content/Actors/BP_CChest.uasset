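; Treasure chest actor that drops items and dissolves away when destroyed.
; SpawnItems runs the parent logic, then spawns a BP_CItemBase at the chest's transform for each SpawnItemID entry, passing the instigator pawn.
; DestroyAction plays a timeline that drives the "Amount" parameter on dynamic materials of the treasure, lid and base meshes, then calls the parent destroy action.
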(event EventBeginPlay)

(event Collision|EventActorBeginOverlap
  (params (OtherActor :type Actor%20Object%20Reference)))

(event EventTick
  (params (DeltaSeconds :type Float%20%28single-precision%29)))

(event EventDestroyAction
  (bind _amount (Timeline|DestroyDissolve PlayFromStart)
    (:Update
      (for _array_element (Rendering|Material|GetMaterials (Variables|Default|GetTreasureMesh))
        (bind _asmaterial_instance_dynamic (Utilities|Casting|CastToMaterialInstanceDynamic _array_element))
        (Rendering|Material|SetScalarParameterValue _asmaterial_instance_dynamic "Amount" _amount :!class /Script/Engine.MaterialInstanceDynamic))
      (for _array_element_2 (Rendering|Material|GetMaterials (Variables|Default|GetLidMesh))
        (bind _asmaterial_instance_dynamic_2 (Utilities|Casting|CastToMaterialInstanceDynamic _array_element_2))
        (Rendering|Material|SetScalarParameterValue _asmaterial_instance_dynamic_2 "Amount" _amount :!class /Script/Engine.MaterialInstanceDynamic))
      (for _array_element_3 (Rendering|Material|GetMaterials (Variables|Default|GetBaseMesh))
        (bind _asmaterial_instance_dynamic_3 (Utilities|Casting|CastToMaterialInstanceDynamic _array_element_3))
        (Rendering|Material|SetScalarParameterValue _asmaterial_instance_dynamic_3 "Amount" _amount :!class /Script/Engine.MaterialInstanceDynamic)))
    (:Finished
      (|CallParentFunction))))

(event EventSpawnItems
  (params (InstigatorPawn :type Pawn%20Object%20Reference))
  (|CallParentFunction InstigatorPawn)
  (for _array_element (Variables|Default|GetSpawnItemID)
    (Game|SpawnActorfromClass "/Game/Actors/Items/BP_CItemBase.BP_CItemBase_C" (Transformation|GetActorTransform) "Undefined" 0 _array_element InstigatorPawn)))

(fn ConstructionScript)