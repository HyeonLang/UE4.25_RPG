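; Player controller for an RPG that creates the main HUD for the local player and handles interaction and inventory keys.
; F forwards to the character's interaction component for primary interaction.
; B toggles a freshly created inventory widget, with SetCursorMode switching the cursor and input mode between game-and-UI and game-only.
; Other keys are debug probes that print item lookups, PlayerState inventory data and authority, or call a game mode test function.
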(event Custom|Test
  (bind _asbp_ue4_rpggame_mode_base (Utilities|Casting|CastToBP_UE4_RPGGameModeBase (Game|GetGameMode))
    (:then
      (Default|TestFunc _asbp_ue4_rpggame_mode_base))
    (:CastFailed
      (Development|PrintString "Hello"))))

(event EventBeginPlay
  (if (Pawn|IsLocalController)
    (bind _returnvalue (UserInterface|CreateWidget "/Game/UI/WB_MainHUD.WB_MainHUD_C" self))
    (UserInterface|Viewport|AddtoViewport _returnvalue 0)))

(event EventTick
  (params (DeltaSeconds :type Float%20%28single-precision%29)))

(event Input|KeyboardEvents|0
  (params (Key :type Key%20Structure :default "None"))
  (:Pressed
    (bind _returnvalue (Class|CItemManager|GetInstance))
    (Development|PrintString (Utilities|String|ToString(Name) (.ItemName (Utilities|Struct|BreakItemInfo (Class|CItemManager|GetItemInfobyID _returnvalue "1001")))))))

(event Input|KeyboardEvents|F
  (params (Key :type Key%20Structure :default "None"))
  (:Pressed
    (Class|CInteractionComponent|PrimaryInteraction (Class|CPlayerCharacter|GetInteractionComponent (Class|CPlayerController|GetPlayerCharacter)))))

(event Input|KeyboardEvents|G
  (params (Key :type Key%20Structure :default "None"))
  (:Pressed
    (bind _ascplayer_state (Utilities|Casting|CastToCPlayerState (Variables|Default|GetPlayerState)))
    (Development|PrintString (Utilities|String|Append "itemlist : Misc" (Utilities|String|ToString(Integer) (Utilities|Map|Length (Variables|/Script/UE4_RPG.CInventory|GetMiscItemList (Class|CPlayerState|GetPlayerInventory _ascplayer_state)))) "  consumable : " (Utilities|String|ToString(Integer) (Utilities|Map|Length (Variables|/Script/UE4_RPG.CInventory|GetConsumableItemList (Class|CPlayerState|GetPlayerInventory _ascplayer_state)))) "  Empty : " (Utilities|String|ToString(Integer) (Utilities|Map|Length (Variables|/Script/UE4_RPG.CInventory|GetMiscItemList (Class|CPlayerState|GetPlayerInventory _ascplayer_state)))) (Utilities|String|ToString(Integer) (.Value (Utilities|Map|Find (Variables|/Script/UE4_RPG.CInventory|GetMiscItemList (Class|CPlayerState|GetPlayerInventory _ascplayer_state)) "1001")))))
    (Development|PrintString (Utilities|String|ToString(Boolean) (.ReturnValue (Utilities|Map|Find (Variables|/Script/UE4_RPG.CInventory|GetMiscItemList (Class|CPlayerState|GetPlayerInventory _ascplayer_state)) "1001"))))))

(event Input|KeyboardEvents|B
  (params (Key :type Key%20Structure :default "None"))
  (:Pressed
    (if (Variables|Default|GetIsInventory)
      (CallFunction|SetCursorMode false)
      (Widget|RemovefromParent (Variables|Default|GetInventoryWidget))
      (Variables|Default|SetIsInventory false)
      (else
        (bind _returnvalue (UserInterface|CreateWidget "/Game/UI/WB_Inventory.WB_Inventory_C" self))
        (bind _output_get (Variables|Default|SetInventoryWidget _returnvalue))
        (UserInterface|Viewport|AddtoViewport _output_get 0)
        (CallFunction|SetCursorMode true)
        (Variables|Default|SetIsInventory true)))))

(event Input|KeyboardEvents|I
  (params (Key :type Key%20Structure :default "None"))
  (:Pressed
    (Development|PrintString (Utilities|String|ToString(Boolean) (Ability|HasAuthority)))
    (CallFunction|Test)))

(fn ConstructionScript)

(fn SetCursorMode
  (params (IsCursorMode :type Boolean))
  (bind _self self)
  (Variables|Default|SetbShowMouseCursor IsCursorMode)
  (if IsCursorMode
    (Input|SetInputModeGameandUI _self 0 "DoNotLock" true)
    (else
      (Input|SetInputModeGameOnly _self))))