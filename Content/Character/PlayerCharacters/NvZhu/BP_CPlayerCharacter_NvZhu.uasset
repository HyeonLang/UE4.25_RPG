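; BP_CPlayerCharacter_NvZhu is the NvZhu player character Blueprint, which adds an on-screen action-system debug readout to its parent class.
; After the parent Tick, DataPrint joins the ActionComp's active gameplay tags into one string and prints it.
; It also prints each running action's name with its current and next combo action names.
; Prints last one frame's delta time and skip the log, forming a live display.
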(event EventBeginPlay)

(event Collision|EventActorBeginOverlap
  (params (OtherActor :type Actor%20Object%20Reference)))

(event EventTick
  (params (DeltaSeconds :type Float%20%28single-precision%29))
  (|CallParentFunction DeltaSeconds)
  (CallFunction|DataPrint DeltaSeconds))

(fn ConstructionScript)

(fn DataPrint
  (params (DeltaTime :type Float%20%28single-precision%29))
  (Utilities|FlowControl|Sequence
    (:then_0
      (for _array_element (.gameplaytags (Variables|/Script/UE4_RPG.CActionComponent|GetActiveGameplayTags (Variables|Default|GetActionComp)))
        (Variables|Default|SetSTR (Utilities|String|Append (Variables|Default|GetSTR) (Utilities|String|ToString(Name) (.returnvalue _array_element)))))
      (Development|PrintString (Variables|Default|GetSTR) true false "(R=1.000000,G=0.000000,B=0.882115,A=1.000000)" DeltaTime)
      (Variables|Default|SetSTR ""))
    (:then_1
      (for _array_element_2 (Class|CActionComponent|GetActions (Variables|Default|GetActionComp))
        (if (Class|CAction|IsRunning _array_element_2)
          (Development|PrintString (Utilities|String|Append (Utilities|GetDisplayName _array_element_2) " " (Utilities|String|ToString(Name) (Variables|/Script/UE4_RPG.CAction|GetCurrentComboActionName _array_element_2)) " " (Utilities|String|ToString(Name) (Variables|/Script/UE4_RPG.CAction|GetNextComboActionName _array_element_2))) true false "(R=1.000000,G=0.314951,B=0.414810,A=1.000000)" DeltaTime))))))