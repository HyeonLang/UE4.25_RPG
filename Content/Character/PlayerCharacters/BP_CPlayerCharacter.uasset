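; BP_CPlayerCharacter is a player character Blueprint that provides forward movement events for dashing and moving toward a target.
; Dash and non-direct MovetoTarget each play their own timeline, spreading MoveLength over swept world offsets scaled by frame time and the timeline's Delta track.
; Direct MovetoTarget applies the whole offset at once, and MovetoTarget ignores non-positive lengths.
; StopMove halts only the Dash timeline.
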(event Custom|StopMove
  (bind _delta (Timeline|타임라인_0 Stop)
    (:Update
      (Transformation|AddActorWorldOffset (* (Transformation|GetActorForwardVector) (* (stale EventDash MoveLength) (/ (Utilities|Time|GetWorldDeltaSeconds) _delta))) true))))

(event EventBeginPlay)

(event Collision|EventActorBeginOverlap
  (params (OtherActor :type Actor%20Object%20Reference)))

(event EventTick
  (params (DeltaSeconds :type Float%20%28single-precision%29)))

(event EventDash
  (params (MoveLength :type Float%20%28single-precision%29))
  (bind _delta (Timeline|타임라인_0 PlayFromStart)
    (:Update
      (Transformation|AddActorWorldOffset (* (Transformation|GetActorForwardVector) (* MoveLength (/ (Utilities|Time|GetWorldDeltaSeconds) _delta))) true))))

(event EventMovetoTarget
  (params (MoveLength :type Float%20%28single-precision%29) (bDirect :type Boolean))
  (if (> MoveLength 0.0)
    (if bDirect
      (Transformation|AddActorWorldOffset (* (Transformation|GetActorForwardVector) MoveLength) true)
      (else
        (bind _delta (Timeline|타임라인_1 PlayFromStart)
          (:Update
            (Transformation|AddActorWorldOffset (* (Transformation|GetActorForwardVector) (* MoveLength (/ (Utilities|Time|GetWorldDeltaSeconds) _delta))) true)))))))

(fn ConstructionScript)