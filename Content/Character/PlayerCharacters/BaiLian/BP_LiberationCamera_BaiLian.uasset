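; Cinematic camera actor for the character BaiLian's Liberation sequence, extending a parent that supplies the PlayCinematic hook.
; PlayCinematic calls the parent, then plays a timeline from the start to drive the CineCamera's focal length and relative location and rotation.
; Camera height is shifted down by a fixed offset from the timeline track.
; When the timeline ends, it calls PlayCinematicFinished.
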(event EventBeginPlay
  (|CallParentFunction) ; 지금 이 노드는 비활성 상태입니다. \n핀을 끌어서 다른 노드를 연결하면 활성화됩니다.
)

(event Collision|EventActorBeginOverlap
  (params (OtherActor :type Actor%20Object%20Reference))
  (|CallParentFunction OtherActor) ; 지금 이 노드는 비활성 상태입니다. \n핀을 끌어서 다른 노드를 연결하면 활성화됩니다.
)

(event EventTick
  (params (DeltaSeconds :type Float%20%28single-precision%29))
  (|CallParentFunction DeltaSeconds) ; 지금 이 노드는 비활성 상태입니다. \n핀을 끌어서 다른 노드를 연결하면 활성화됩니다.
)

(event EventPlayCinematic
  (bind _cinecameracomp (Variables|Default|GetCineCameraComp))
  (|CallParentFunction)
  (bind (_direction _focallength _location _rotation) (Timeline|Lib_CameraAction_BaiLian PlayFromStart)
    (:Update
      (Variables|/Script/CinematicCamera.CineCameraComponent|SetCurrentFocalLength _cinecameracomp _focallength)
      (Transformation|SetRelativeLocationAndRotation _cinecameracomp (Math|Vector|MakeVector (.x _location) (.y _location) (- (.z _location) 88.0)) (Math|Rotator|MakeRotator (.x _rotation) (.y _rotation) (.z _rotation)) false false))
    (:Finished
      (Class|CPlayerCineCameraActor|PlayCinematicFinished))))

(fn ConstructionScript
  (|CallParentFunction))