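; Spawned effect actor for BaiLian's resonance skill, showing the skill effect and driving its repeated and final attacks through OwnerAction.
; BeginPlay applies the effect template and transform from the action's current combo data, scales it via timeline, then starts a looping attack timer.
; OffEffect stops the timer, runs a second scale timeline, spawns the closing emitter, fires a last attack and destroys the actor.
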(event Custom|OnEffect
  (Variables|Default|SetInitialEffectScale (Transformation|GetWorldScale (Variables|Default|GetEffectComp)))
  (bind _delta (Timeline|타임라인_1 PlayFromStart)
    (:Update
      (Transformation|SetWorldScale3D (Variables|Default|GetEffectComp) (* (Variables|Default|GetInitialEffectScale) _delta)))
    (:Finished
      (bind _returnvalue (Utilities|Time|SetTimerbyEvent (delegate Custom|IntervalAttack) (Variables|Default|GetAttackInterval) true))
      (Variables|Default|SetIntervalAttackTimerHandle _returnvalue))))

(event Custom|OffEffect
  (bind _owneraction (Variables|Default|GetOwnerAction))
  (bind _intervalattacktimerhandle (Variables|Default|GetIntervalAttackTimerHandle))
  (bind _owneraction_2 (Variables|Default|GetOwnerAction))
  (bind _comboindex (Variables|/Script/UE4_RPG.CActionBase|GetComboIndex _owneraction_2))
  (bind _actiondatas (Variables|/Script/UE4_RPG.CActionBase|GetActionDatas _owneraction_2))
  (bind _output (Utilities|Array|Get(acopy) _actiondatas _comboindex))
  (bind _output_2 (Utilities|Array|Get(acopy) (.effectdatas _output) 1))
  (if (Utilities|Time|IsValidTimerHandle _intervalattacktimerhandle)
    (Utilities|Time|ClearandInvalidateTimerbyHandle _intervalattacktimerhandle))
  (Variables|Default|SetInitialEffectScale (Transformation|GetWorldScale (Variables|Default|GetEffectComp)))
  (bind _delta (Timeline|타임라인_0 PlayFromStart)
    (:Update
      (Transformation|SetWorldScale3D (Variables|Default|GetEffectComp) (* (Variables|Default|GetInitialEffectScale) _delta)))
    (:Finished
      (Utilities|IsValid _owneraction_2
        (:Is%20Valid
          (Effects|SpawnEmitteratLocation (.effects _output_2) (Transformation|GetActorLocation) "0, 0, 0" (.scale (.effecttransform _output_2)))
          (Utilities|IsValid _owneraction
            (:Is%20Valid
              (bind _ascharacter (Utilities|Casting|CastToCharacter (Components|GetOwner (Class|CAction|GetOwningComponent _owneraction))))
              (Class|CActionBase|AttackElapsed _owneraction _ascharacter 3)
              (Actor|DestroyActor))))))))

(event Custom|IntervalAttack
  (bind _owneraction (Variables|Default|GetOwnerAction))
  (Utilities|IsValid _owneraction
    (:Is%20Valid
      (bind _ascharacter (Utilities|Casting|CastToCharacter (Components|GetOwner (Class|CAction|GetOwningComponent _owneraction))))
      (Class|CActionBase|AttackElapsed _owneraction _ascharacter))))

(event EventBeginPlay
  (bind _owneraction (Variables|Default|GetOwnerAction))
  (bind _actiondatas (Variables|/Script/UE4_RPG.CActionBase|GetActionDatas _owneraction))
  (bind _comboindex (Variables|/Script/UE4_RPG.CActionBase|GetComboIndex _owneraction))
  (bind _output (Utilities|Array|Get(acopy) _actiondatas _comboindex))
  (bind _effectdatas (Utilities|Struct|BreakActionData _output))
  (bind _output_2 (Utilities|Array|Get(acopy) _effectdatas))
  (Utilities|IsValid _owneraction
    (:Is%20Valid
      (Effects|Components|ParticleSystem|SetTemplate (Variables|Default|GetEffectComp) (.effects _output_2))
      (Transformation|SetRelativeTransform (Variables|Default|GetEffectComp) (.effecttransform _output_2) false true)
      (CallFunction|OnEffect))))

(event Collision|EventActorBeginOverlap
  (params (OtherActor :type Actor%20Object%20Reference)))

(event EventTick
  (params (DeltaSeconds :type Float%20%28single-precision%29)))

(fn ConstructionScript)