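; Lobby game mode that sets up character display and camera, and runs a hard-coded database test.
; On BeginPlay it connects to a local database through the CGameInstance's DBManager and inserts a test user; the Disconnect call is never executed.
; Each PostLogin spawns a ChangLi lobby character, spaced along Y by player count.
; It then points player controller 0, not necessarily the joining player, at the first BP_LobbyCamera found.
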(event EventBeginPlay
  (bind _ascgame_instance (Utilities|Casting|CastToCGameInstance (Game|GetGameInstance))
    (:then
      (bind _dbmanager (Variables|/Script/UE4_RPG.CGameInstance|GetDBManager _ascgame_instance)
        (:then
          (bind _returnvalue (Class|CDBManager|Connect _dbmanager "127.0.0.1" 33060 "root" "1234" "testdb"))
          (if _returnvalue
            (Class|CDBManager|InsertUserTable _dbmanager "usertable" "aaa" "111")))
        (:else
          (Development|PrintString "no dbmanager"))))
    (:CastFailed
      (Development|PrintString "no instance"))))

(event EventPostLogin
  (params (NewPlayer :type Player%20Controller%20Object%20Reference))
  (Game|SpawnActorfromClass "/Game/Character/PlayerCharacters/ChangLi/BP_LobbyCharacter_ChangLi.BP_LobbyCharacter_ChangLi_C" (Math|Transform|MakeTransform (Math|Vector|MakeVector 0.0 (+ (* (Variables|Default|GetNumberOfPlayers) 1.5e+02) -1.5e+02) 0.0) "0,-180.000000, 0") "Undefined" 0 0)
  (bind _outactors (Actor|GetAllActorsOfClass "/Game/Actors/BP_LobbyCamera.BP_LobbyCamera_C"))
  (bind _array_element (Utilities|Array|ForEachLoopwithBreak _outactors :!label _label)
    (:LoopBody
      (Game|Player|SetViewTargetwithBlend (Game|GetPlayerController 0) _array_element 0.0 "VTBlend_Linear" 0.0 false)
      (goto _label Break))))

(fn ConstructionScript)